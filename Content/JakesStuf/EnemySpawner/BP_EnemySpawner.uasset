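; Enemy spawner actor that spawns one or two BP_NPC_1 enemies at its location on BeginPlay.
; The Ranged flag sets the base type, with true giving Saber and false giving Ranged.
; Chances read from BP_SlimeInstance roll for a double spawn, then per enemy for a tier upgrade.
; Upgrades randomly pick between two variants for the base type, while failed rolls spawn the base type.
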(event `self.ReceiveBeginPlay`
  (bind _returnvalue (> (`KismetMathLibrary.RandomInteger` 100) 50))
  (bind _returnvalue_2 (`KismetMathLibrary.Conv_VectorToTransform` (`SceneComponent.K2_GetComponentLocation` (`self.DefaultSceneRoot`))))
  (if (`self.Ranged?`)
    (set `self.EnemyType` "NewEnumerator0")
    (else
      (set `self.EnemyType` "NewEnumerator1")))
  (bind _asbp_slime_instance (cast `/Game/TwinStickBP/BP_SlimeInstance` (`GameplayStatics.GetGameInstance`)))
  (if (< (`KismetMathLibrary.RandomInteger` 100) (`/Game/TwinStickBP/BP_SlimeInstance.DoubleSpawnChance` _asbp_slime_instance))
    (for _ (range 2)
      (if (< (`KismetMathLibrary.RandomInteger` 100) (`/Game/TwinStickBP/BP_SlimeInstance.Up-TierChance` _asbp_slime_instance)) :!label _label
        (switch `/Game/AI/NPC/FolowRanged/NPC-Type` (`self.EnemyType`)
          (:`NewEnumerator0`
            (if _returnvalue
              (`|SpawnActorFromClass` "/Game/AI/NPC/BP_NPC_1.BP_NPC_1_C" _returnvalue_2 "AdjustIfPossibleButAlwaysSpawn" "OverrideRootScale" null true "NewEnumerator6" 1.0 20.0 15.0 null)
              (else
                (`|SpawnActorFromClass` "/Game/AI/NPC/BP_NPC_1.BP_NPC_1_C" _returnvalue_2 "AdjustIfPossibleButAlwaysSpawn" "OverrideRootScale" null true "NewEnumerator7" 1.0 20.0 15.0 null))))
          (:`NewEnumerator1`
            (if _returnvalue
              (`|SpawnActorFromClass` "/Game/AI/NPC/BP_NPC_1.BP_NPC_1_C" _returnvalue_2 "AdjustIfPossibleButAlwaysSpawn" "OverrideRootScale" null true "NewEnumerator2" 1.0 20.0 15.0 null)
              (else
                (`|SpawnActorFromClass` "/Game/AI/NPC/BP_NPC_1.BP_NPC_1_C" _returnvalue_2 "AdjustIfPossibleButAlwaysSpawn" "OverrideRootScale" null true "NewEnumerator8" 1.0 20.0 15.0 null)))))
        (else
          (`|SpawnActorFromClass` "/Game/AI/NPC/BP_NPC_1.BP_NPC_1_C" (`KismetMathLibrary.Conv_VectorToTransform` (`SceneComponent.K2_GetComponentLocation` (`self.DefaultSceneRoot`))) "AdjustIfPossibleButAlwaysSpawn" "OverrideRootScale" null true (`self.EnemyType`) 1.0 20.0 15.0 null))))
    (else
      (goto _label))))

(fn `UserConstructionScript`)