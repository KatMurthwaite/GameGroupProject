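; Cube-bodied AI enemy NPC that chases, deals repeated contact damage to the player, and bursts into healing slime chunks on death.
; AI perception writes sight and target to the blackboard; while locked on, melee NPCs copy the enemy's location into a looping AIMoveTo.
; Construction and SetSize fit the capsule to the cube's scale.
; Movement and timeline dash input handlers are also present; aiming and shooting nodes are disconnected.
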(event `self.ReceiveBeginPlay`
  ;[1 1 1] Movement
  (`|ExecutionSequence`
    (:`then_0`
      (`|AIMoveTo` self (`self.Destination`) null :!label _label
        (:`then`
          (`KismetSystemLibrary.Delay` 0.2)
          (goto _label))))))

(event `self.ReceiveTick`
  (params (DeltaSeconds :type "Float (single-precision)"))
  (`|ExecutionSequence`
    (:`then_0`
      (`/Engine/EditorBlueprintResources/StandardMacros.Gate` (`self.EnemyLock`)
        (:`Exit`
          (bind _enemy_actor (`self.Enemy Actor`)
            (:`then`
              (bind _output_get (set `self.AimLocation` (`self.K2_GetActorLocation` _enemy_actor)))
              ;[1 1 1] Follow for all melee
              (if (`self.Melee?`)
                (set `self.Destination` _output_get)))
            (:`else`)))))))

(event `InputAction|Jump`
  (params (Key :type "Key Structure"))
  (bind (_returnvalue_x _returnvalue_y) (`KismetMathLibrary.BreakVector` (`self.GetLastMovementInputVector`)))
  (:`Pressed`
    (if (or (!= _returnvalue_x 0.0) (!= _returnvalue_y 0.0))
      (if (`self.CanDash`)
        (set `self.CanDash` false)
        (set `self.DashDir` (`self.GetLastMovementInputVector`))
        (set `self.DashStart` (`SceneComponent.K2_GetComponentLocation` (`self.CapsuleComponent`)))
        (bind (_direction _dishydashy) (`Timeline|DashTimeline` :!via `PlayFromStart`)
          (:`Update`
            (`SceneComponent.K2_SetWorldLocation` (`self.CapsuleComponent`) (+ (* (* (`self.DashDir`) (`self.Dash length`)) _dishydashy) (`self.DashStart`)) true false))
          (:`Finished`
            (`KismetSystemLibrary.Delay` 0.3)
            (set `self.CanDash` true)))))))

(event `InputAxis|MoveForward`
  (params (AxisValue :type "Float (single-precision)"))
  ;[1 1 1] Movement
  (`self.AddMovementInput` (70.0 0.0 0.0) AxisValue))

(event `InputAxis|MoveRight`
  (params (AxisValue :type "Float (single-precision)"))
  ;[1 1 1] Movement
  (`self.AddMovementInput` (0.0 70.0 0.0) AxisValue))

(event `self.ReceiveAnyDamage`
  (params (Damage :type "Float (single-precision)") (DamageType :type "DamageType Object Reference") (InstigatedBy :type "Controller Object Reference") (DamageCauser :type "Actor Object Reference"))
  ;[1 1 1] Receive damage
  (bind _dead (`self.Damaged` Damage))
  (if _dead
    (`self.Death`)))

(event `self.DamageBox.OnComponentBeginOverlap`
  (params (OverlappedComponent :type "PrimitiveComponent Object Reference") (OtherActor :type "Actor Object Reference") (OtherComp :type "PrimitiveComponent Object Reference") (OtherBodyIndex :type Integer) (bFromSweep :type Boolean) (SweepResult :type "HitResult Structure (by ref)"))
  (bind _returnvalue (`ActorComponent.GetOwner` OtherComp))
  ;[1 1 1] Melee
  (`/Engine/EditorBlueprintResources/StandardMacros.IsValid` OtherComp
    (:`Is Valid`
      (if (`self.PlayerOverlap`)
        _
        (elif (`self.ActorHasTag` _returnvalue "Player")
          (set `self.PlayerOverlap` true)
          (`GameplayStatics.ApplyDamage` _returnvalue (`self.ProximityDamageAmount`) :!label _label_2)
          (`/Engine/EditorBlueprintResources/StandardMacros.Gate` (`self.PlayerOverlap`)
            (:`Exit`
              (`KismetSystemLibrary.PrintString` "Overlap damage")
              (`KismetSystemLibrary.Delay` 2.0)
              (`/Engine/EditorBlueprintResources/StandardMacros.IsValid` (stale `self.DamageBox.OnComponentEndOverlap` OtherComp)
                (:`Is Valid`
                  (goto _label_2))))))))))

(event `self.DamageBox.OnComponentEndOverlap`
  (params (OverlappedComponent :type "PrimitiveComponent Object Reference") (OtherActor :type "Actor Object Reference") (OtherComp :type "PrimitiveComponent Object Reference") (OtherBodyIndex :type Integer))
  ;[1 1 1] Melee
  (`/Engine/EditorBlueprintResources/StandardMacros.IsValid` OtherComp
    (:`Is Valid`
      (if (`self.ActorHasTag` (`ActorComponent.GetOwner` OtherComp) "Player")
        (set `self.PlayerOverlap` false)))))

(event `self.AIPerception.OnTargetPerceptionUpdated`
  (params (Actor :type "Actor Object Reference") (Stimulus :type "AIStimulus Structure"))
  (bind _returnvalue (`AIBlueprintHelperLibrary.GetBlackboard` self))
  ;[1 1 1] Sight
  (`BlackboardComponent.SetValueAsBool` _returnvalue "CanSee" Stimulus_bSuccessfullySensed)
  (`BlackboardComponent.SetValueAsObject` _returnvalue "TargetActor" Actor)
  (set `self.Enemy Actor` Actor))

(fn `Damaged`
  (params (Amount :type "Float (double-precision)"))
  (returns (Dead :type Boolean))
  (bind _returnvalue (- (`self.Health`) Amount))
  (bind _returnvalue_2 (<= _returnvalue 0.0))
  (if (not _returnvalue_2)
    (set `self.Health` _returnvalue))
  (return _returnvalue_2))

(fn `Death`
  (`KismetSystemLibrary.PrintString` "Dead")
  (for _ (range (+ (+ (`KismetMathLibrary.RandomInteger` 10) 5) 1))
    (bind _returnvalue (`|SpawnActorFromClass` "/Game/TwinStickBP/Blueprints/HealingSlimeChunk.HealingSlimeChunk_C" (`KismetMathLibrary.MakeTransform` (+ (`SceneComponent.K2_GetComponentLocation` (`self.Cube`)) (`KismetMathLibrary.MakeVector` (`KismetMathLibrary.RandomFloatInRange` 0.0 40.0) (`KismetMathLibrary.RandomFloatInRange` 0.0 40.0) (`KismetMathLibrary.RandomFloatInRange` 0.0 40.0))) (struct) (0.2 0.2 0.2)) "Undefined" "OverrideRootScale" null null))
    (`PrimitiveComponent.AddImpulse` (`/Game/TwinStickBP/Blueprints/HealingSlimeChunk.Sphere` _returnvalue) (+ (`KismetMathLibrary.MakeVector` (`KismetMathLibrary.RandomFloatInRange` 0.0 40.0) (`KismetMathLibrary.RandomFloatInRange` 0.0 40.0) (`KismetMathLibrary.RandomFloatInRange` 0.0 40.0)) (`self.GetVelocity`)) "None" false))
  (`self.K2_DestroyActor`))

(fn `FaceEnemy`
  (set `self.AimLocation` (`self.K2_GetActorLocation` (`self.Enemy Actor`))))

(fn `LockOnEnemy`
  (set `self.EnemyLock` true))

(fn `Set Size`
  (params (`Size of cube` :type "Float (double-precision)"))
  (returns (NewParam :type "Float (double-precision)"))
  (locals (NewLocalVar_0 :type "Vector Structure" :default (0.0 0.0 0.0)) (NewLocalVar_1 :type "Vector Structure" :default (0.0 0.0 0.0)))
  (bind _capsulecomponent (`self.CapsuleComponent`))
  (bind _relativescale3d_x (`KismetMathLibrary.BreakVector` (`SceneComponent.RelativeScale3D` (`self.Cube`))))
  (bind _returnvalue (* (/ _relativescale3d_x 2.0) 100.0))
  (`SceneComponent.SetRelativeScale3D` (`self.Cube`) (`KismetMathLibrary.MakeVector` `Size of cube` `Size of cube` `Size of cube`))
  (`CapsuleComponent.SetCapsuleHalfHeight` _capsulecomponent _returnvalue true)
  (`CapsuleComponent.SetCapsuleRadius` _capsulecomponent _returnvalue true))

(fn `SetDestination`
  (params (Destination :type "Vector Structure"))
  (set `self.Destination` Destination))

(fn `UnlockEnemy`
  (set `self.EnemyLock` false))

(fn `UserConstructionScript`
  (bind _capsulecomponent (`self.CapsuleComponent`))
  (bind _relativescale3d_x (`KismetMathLibrary.BreakVector` (`SceneComponent.RelativeScale3D` (`self.Cube`))))
  (bind _returnvalue (* (/ _relativescale3d_x 2.0) 100.0))
  (`CapsuleComponent.SetCapsuleHalfHeight` _capsulecomponent _returnvalue true)
  (`CapsuleComponent.SetCapsuleRadius` _capsulecomponent _returnvalue true))