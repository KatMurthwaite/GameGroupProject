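; NPC character Blueprint that exposes a command and query interface for an AI-driven, armed NPC.
; Action events forward stance, gait, aiming, weapon switching, firing and ammo to the ACALS locomotion and ACWCS weapon components, with AIMoveTo handling movement.
; Look and aim events blend rotations through timelines, via ACALS or the AI controller's control rotation.
; Getters report health, state, ammo and weapon data; damage destroys the actor at zero health.
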(event `/Game/Common/BPI_Character.ChangeWeapons`
  (params (Slot :type Integer))
  (bind _ac_wcs (`self.AC_WCS`))
  ;[1 1 1] Change Weapon
  (if (!= (`/Game/WeaponSystem/Blueprints/AC_WCS.Current Index` _ac_wcs) Slot)
    (`/Game/WeaponSystem/Blueprints/AC_WCS.Switch Weapon` _ac_wcs Slot)
    (set `self.IsShooting` false)))

(event `/Game/Common/BPI_Character.LookAtDirection`
  (params (Direction :type "Rotator Structure"))
  (bind _ac_als (`self.AC_ALS`))
  (bind _lookingrotation (`/Game/ALS/Blueprints/AC_ALS.LookingRotation` _ac_als))
  ;[1 1 1] Look at direction
  (bind (_direction _newtrack_1) (`Timeline|Timeline_0`)
    (:`Update`
      (`/Game/ALS/Blueprints/AC_ALS.SetCharacterRotation` _ac_als (`KismetMathLibrary.RLerp` _lookingrotation (`KismetMathLibrary.MakeRotator` (.roll _lookingrotation) (.pitch _lookingrotation) (.yaw Direction)) _newtrack_1 true) false 1.0))))

(event `/Game/Common/BPI_Character.PullTrigger`
  ;[1 1 1] Pull/Release Trigger
  (`/Game/WeaponSystem/Blueprints/AC_WCS.Pull Trigger` (`self.AC_WCS`) true)
  (set `self.IsShooting` true))

(event `/Game/Common/BPI_Character.AimDownSight`
  (params (ShouldAim :type Boolean))
  ;[1 1 1] Aim Down Sight
  (`/Game/ALS/Blueprints/AC_ALS.Set ALS_Aiming Event ( SERVER )` (`self.AC_ALS`) ShouldAim)
  (`/Game/WeaponSystem/Blueprints/AC_WCS.Aim` (`self.AC_WCS`) ShouldAim))

(event `/Game/Common/BPI_Character.ReleaseTrigger`
  ;[1 1 1] Pull/Release Trigger
  (`/Game/WeaponSystem/Blueprints/AC_WCS.Pull Trigger` (`self.AC_WCS`) false)
  (set `self.IsShooting` false))

(event `/Game/Common/BPI_Character.SetMovementMode`
  (params (Movement_Mode :type "/Game/ALS/Blueprints/Enums/ALS_Gait Enum" :default "NewEnumerator0"))
  ;[1 1 1] Set Movement mode
  (`/Game/ALS/Blueprints/AC_ALS.Set ALS_Gait Event` (`self.AC_ALS`) Movement_Mode))

(event `/Game/Common/BPI_Character.LookAtPosition`
  (params (Position :type "Vector Structure"))
  (bind _ac_als (`self.AC_ALS`))
  (bind _lookingrotation (`/Game/ALS/Blueprints/AC_ALS.LookingRotation` _ac_als))
  ;[1 1 1] LookAtPosition
  (bind (_direction _newtrack_1) (`Timeline|Timeline_2`)
    (:`Update`
      (`/Game/ALS/Blueprints/AC_ALS.SetCharacterRotation` _ac_als (`KismetMathLibrary.RLerp` _lookingrotation (`KismetMathLibrary.MakeRotator` (.roll _lookingrotation) (.pitch _lookingrotation) (.yaw (`KismetMathLibrary.FindLookAtRotation` (`self.K2_GetActorLocation` self) Position))) _newtrack_1 true) false 1.0))))

(event `/Game/Common/BPI_Character.SetStance`
  (params (Stance :type "/Game/ALS/Blueprints/Enums/ALS_Stance Enum" :default "NewEnumerator0"))
  ;[1 1 1] Set Stance
  (`/Game/ALS/Blueprints/AC_ALS.Set ALS_Stance Event` (`self.AC_ALS`) Stance))

(event `/Game/Common/BPI_Character.MoveTo`
  (params (Destination :type "Vector Structure"))
  ;[1 1 1] Move to
  (set `self.IsMoving` true)
  (`|AIMoveTo` self Destination null
    (:`OnSuccess`
      _)
    (:`OnFail`
      _))
  (set `self.IsMoving` false))

(event `/Game/Common/BPI_Character.AimAtPosition`
  (params (Position :type "Vector Structure"))
  (bind _ac_als (`self.AC_ALS`))
  ;[1 1 1] AimAtPosition
  (bind _direction (message `/Game/Common/BPI_Character.GetAimingDirection` _ac_als))
  (bind (_direction_2 _newtrack_1) (`Timeline|Timeline_3`)
    (:`Update`
      (`/Game/ALS/Blueprints/AC_ALS.Set LookingRotation Event ( SERVER )` _ac_als (`KismetMathLibrary.RLerp` _direction (`KismetMathLibrary.FindLookAtRotation` (`self.K2_GetActorLocation` self) Position) _newtrack_1 true)))))

(event `self.ReceiveTick`
  (params (DeltaSeconds :type "Float (single-precision)"))
  ;[1 1 1] AimAtPosition
)

(event `/Game/Common/BPI_Character.AimAtDirection`
  (params (Direction :type "Rotator Structure"))
  (bind _returnvalue (`AIBlueprintHelperLibrary.GetAIController` self))
  (bind _lookingrotation (`/Game/ALS/Blueprints/AC_ALS.LookingRotation` (`self.AC_ALS`)))
  (bind _returnvalue_2 (`KismetMathLibrary.MakeRotator` (.roll _lookingrotation) (.pitch _lookingrotation) (.yaw Direction)))
  ;[1 1 1] Aim At Direction
  (bind (_direction _newtrack_1) (`Timeline|Timeline_1`)
    (:`Update`
      (`Controller.SetControlRotation` _returnvalue (`KismetMathLibrary.RLerp` _lookingrotation _returnvalue_2 _newtrack_1 true)))
    (:`Finished`
      (`Controller.SetControlRotation` _returnvalue _returnvalue_2))))

(event `self.ReceiveAnyDamage`
  (params (Damage :type "Float (single-precision)") (DamageType :type "DamageType Object Reference") (InstigatedBy :type "Controller Object Reference") (DamageCauser :type "Actor Object Reference"))
  ;[1 1 1] Damaged
  (bind _output_get (set `self.Health` (- (`self.Health`) Damage)))
  (if (<= _output_get 0.0)
    (`self.K2_DestroyActor`)))

(event `/Game/Common/BPI_Character.AddAmmo`
  (params (Type :type "/Game/WeaponSystem/Blueprints/E_AmmoTypes Enum" :default "NewEnumerator6") (Amount :type Integer))
  (bind _ammo (`/Game/WeaponSystem/Blueprints/AC_WCS.Ammo` (`self.AC_WCS`)))
  (bind _value (`BlueprintMapLibrary.Map_Find` _ammo Type))
  ;[1 1 1] Add ammo
  (`KismetSystemLibrary.PrintString` (`KismetStringLibrary.Conv_IntToString` _value))
  (`BlueprintMapLibrary.Map_Add` _ammo Type (+ Amount _value))
  (`KismetSystemLibrary.PrintString` (`KismetStringLibrary.Conv_IntToString` (`BlueprintMapLibrary.Map_Find` _ammo Type))))

(fn `AimToward`)

(fn `AmmoCountOfType`
  (params (AmmoType :type "/Game/WeaponSystem/Blueprints/E_AmmoTypes Enum" :default "NewEnumerator6"))
  (returns (Possible :type Boolean) (AmmoCount :type Integer))
  (bind (_value _returnvalue) (`BlueprintMapLibrary.Map_Find` (`/Game/WeaponSystem/Blueprints/AC_WCS.Ammo` (`self.AC_WCS`)) AmmoType))
  ;[1 1 1] Get ammo count of type
  (return _returnvalue _value))

(fn `CurrentHealth`
  (returns (Health :type "Float (double-precision)"))
  (return (`self.Health`)))

(fn `CurrentState`
  (returns (IsMoving :type Boolean) (IsShooting :type Boolean) (Health :type "Float (double-precision)") (WeaponIndex :type Integer))
  (return (`self.IsMoving`) (`self.IsShooting`) (`self.Health`) (`/Game/WeaponSystem/Blueprints/AC_WCS.Current Index` (`self.AC_WCS`))))

(fn `GetAimingDirection`
  (returns (Direction :type "Rotator Structure"))
  (return (`/Game/ALS/Blueprints/AC_ALS.LookingRotation` (`self.AC_ALS`))))

(fn `GetClipAmmoCount`
  (returns (AmmoCount :type Integer))
  (return (`/Game/WeaponSystem/Blueprints/BP_Weapon.Clip Ammo` (`/Game/WeaponSystem/Blueprints/AC_WCS.Current Weapon` (`self.AC_WCS`)))))

(fn `GetFireMode`
  (returns (FireMode :type "/Game/WeaponSystem/Blueprints/E_FireModes Enum"))
  (return (`/Game/WeaponSystem/Blueprints/BP_Weapon.Fire Mode` (`/Game/WeaponSystem/Blueprints/AC_WCS.Current Weapon` (`self.AC_WCS`)))))

(fn `GetMovementMode`
  (returns (NewParam :type "/Game/ALS/Blueprints/Enums/ALS_Gait Enum"))
  (return (`/Game/ALS/Blueprints/AC_ALS.ALS_Gait` (`self.AC_ALS`))))

(fn `GetRecoilStatus`
  (returns (RecoilStatus :type "Vector2D Structure"))
  (bind _holder (`/Game/WeaponSystem/Blueprints/AC_WCS.Holder` (`self.AC_WCS`)))
  (return (`KismetMathLibrary.MakeVector2D` (`/Game/WeaponSystem/Blueprints/BP_Holder.Temp Yaw` _holder) (`/Game/WeaponSystem/Blueprints/BP_Holder.Temp Pitch` _holder))))

(fn `SelfLocation`
  (returns (Location :type "Vector Structure"))
  (return (`/Game/ALS/Blueprints/AC_ALS.RagdollLocation` (`self.AC_ALS`))))

(fn `SetFireMode`
  (params (FireMode :type "/Game/WeaponSystem/Blueprints/E_FireModes Enum" :default "NewEnumerator0"))
  (returns (Success :type Boolean))
  (bind _output_get (set `/Game/WeaponSystem/Blueprints/BP_Weapon.Fire Mode` FireMode (`/Game/WeaponSystem/Blueprints/AC_WCS.Current Weapon` (`self.AC_WCS`))))
  (return (`|EnumEquality` _output_get FireMode)))

(fn `UserConstructionScript`
  (`parent.UserConstructionScript`))

(fn `WeaponInfo`
  (params (Slot :type Integer))
  (returns (WeaponInfo :type "/Game/WeaponSystem/Blueprints/ST_WeraponAttributes Structure"))
  (return (`/Game/WeaponSystem/Blueprints/BP_Weapon.Weapon Attributes` (`|GetArrayItem` (`/Game/WeaponSystem/Blueprints/AC_WCS.Weapons` (`self.AC_WCS`)) Slot))))